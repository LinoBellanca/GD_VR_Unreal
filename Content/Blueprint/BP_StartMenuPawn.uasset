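; VR-style start menu pawn that lets the player point at and click UMG widgets with either hand.
; Left and right grab inputs press and release a virtual left mouse button on that hand's WidgetInteraction component.
; Each tick, both hands' pointer spline meshes are destroyed and recreated from hand to hit point, only while over a hit-testable widget.
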(event Input|EnhancedActionEvents|EnhancedInputActionIA_Grab_Left
  (params (ActionValue :type Float%20%28double-precision%29) (ElapsedSeconds :type Float%20%28double-precision%29) (TriggeredSeconds :type Float%20%28double-precision%29) (InputAction :type Input%20Action%20Object%20Reference :default "/Game/VRTemplate/Input/Actions/IA_Grab_Left.IA_Grab_Left"))
  (bind _widgetinteractionleft (Variables|Default|GetWidgetInteractionLeft))
  (:Triggered
    (Class|WidgetInteractionComponent|PressPointerKey _widgetinteractionleft "LeftMouseButton"))
  (:Completed
    (Class|WidgetInteractionComponent|ReleasePointerKey _widgetinteractionleft "LeftMouseButton")))

(event Input|EnhancedActionEvents|EnhancedInputActionIA_Grab_Right
  (params (ActionValue :type Float%20%28double-precision%29) (ElapsedSeconds :type Float%20%28double-precision%29) (TriggeredSeconds :type Float%20%28double-precision%29) (InputAction :type Input%20Action%20Object%20Reference :default "/Game/VRTemplate/Input/Actions/IA_Grab_Right.IA_Grab_Right"))
  (bind _widgetinteractionright (Variables|Default|GetWidgetInteractionRight))
  (:Triggered
    (Class|WidgetInteractionComponent|PressPointerKey _widgetinteractionright "LeftMouseButton"))
  (:Completed
    (Class|WidgetInteractionComponent|ReleasePointerKey _widgetinteractionright "LeftMouseButton")))

(event EventTick
  (params (DeltaSeconds :type Float%20%28single-precision%29))
  (CallFunction|WidgetInteractionPointer))

(fn ConstructionScript)

(fn WidgetInteractionPointer
  (bind _widgetinteractionleft (Variables|Default|GetWidgetInteractionLeft))
  (bind _widgetinteractionright (Variables|Default|GetWidgetInteractionRight))
  (bind _returnvalue (Transformation|GetWorldLocation _widgetinteractionright))
  (bind _returnvalue_2 (Transformation|GetWorldLocation _widgetinteractionleft))
  (bind _returnvalue_3 (Class|WidgetInteractionComponent|GetLastHitResult _widgetinteractionleft))
  (bind _returnvalue_4 (Class|WidgetInteractionComponent|GetLastHitResult _widgetinteractionright))
  (bind _returnvalue_5 (Math|Rotator|FindLookatRotation _returnvalue_2 (.location _returnvalue_3)))
  (bind _returnvalue_6 (Math|Rotator|FindLookatRotation _returnvalue (.location _returnvalue_4)))
  (bind _returnvalue_7 (Math|Vector|GetForwardVector _returnvalue_5))
  (bind _returnvalue_8 (Math|Vector|GetForwardVector _returnvalue_6))
  (Utilities|FlowControl|Sequence
    (:then_0
      ;[1 1 1] Sélectionner avec la main gauche
      (bind _leftsplinemesh (Variables|Default|GetLeftSplineMesh)
        (:then
          (Components|DestroyComponent _leftsplinemesh))
        (:else
          _))
      (if (Class|WidgetInteractionComponent|IsOverHitTestVisibleWidget _widgetinteractionleft)
        (bind _returnvalue_9 (AddComponent|AddSplineMeshComponent true))
        (bind _output_get (Variables|Default|SetLeftSplineMesh _returnvalue_9))
        (SplineMesh|SetStartandEnd _output_get _returnvalue_2 _returnvalue_7 (.location _returnvalue_3) (* _returnvalue_7 (Math|Conversions|ToVector(Float) -1.0)) true :!class /Script/Engine.SplineMeshComponent)))
    (:then_1
      ;[1 1 1] Sélectionner avec la main droite
      (bind _rightsplinemesh (Variables|Default|GetRightSplineMesh)
        (:then
          (Components|DestroyComponent _rightsplinemesh))
        (:else
          _))
      (if (Class|WidgetInteractionComponent|IsOverHitTestVisibleWidget _widgetinteractionright)
        (bind _returnvalue_10 (AddComponent|AddSplineMeshComponent true))
        (bind _output_get_2 (Variables|Default|SetRightSplineMesh _returnvalue_10))
        (SplineMesh|SetStartandEnd _output_get_2 _returnvalue _returnvalue_8 (.location _returnvalue_4) (* _returnvalue_8 (Math|Conversions|ToVector(Float) -1.0)) true :!class /Script/Engine.SplineMeshComponent)))))