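; BP_GrabExt is a grabbable VR handle that resizes the sphere of a referenced BP_PlanetPhysics planet.
; On grab, it records its distance to the planet and the sphere's current world scale.
; While held, Tick multiplies that scale by the ratio of current to initial distance, clamping each axis between Min and Max.
; On release, scaling stops and it re-attaches to the MotionController, snapping location while keeping world rotation and scale.
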(event OnGrabbed(GrabComponent)
  (Variables|Default|SetIs%20grabbed%20? true)
  (Variables|Default|SetdistanceOrigine (Math|Vector|VectorLength (- (Transformation|GetActorLocation) (Transformation|GetActorLocation (Variables|Default|GetAs%20BP%20Planet%20Physics)))))
  (Variables|Default|SetOrigin%20Scale (Transformation|GetWorldScale (Variables|/Game/Blueprint/BP_PlanetPhysics.BP_PlanetPhysics_C|GetSphere (Variables|Default|GetAs%20BP%20Planet%20Physics)))))

(event OnDropped(GrabComponent)
  (Variables|Default|SetIs%20grabbed%20? false)
  (Transformation|AttachComponentToComponent (Variables|Default|GetMotion%20Controller) "None" "SnapToTarget" "KeepWorld" "KeepWorld" true))

(event EventTick
  (params (DeltaSeconds :type Float%20%28single-precision%29))
  (bind _returnvalue (Transformation|GetActorLocation))
  (bind _as_bp_planet_physics (Variables|Default|GetAs%20BP%20Planet%20Physics))
  (bind _origin_scale (Variables|Default|GetOrigin%20Scale))
  (bind _distanceorigine (Variables|Default|GetdistanceOrigine))
  (bind _returnvalue_2 (Transformation|GetActorLocation _as_bp_planet_physics))
  (bind _returnvalue_3 (- _returnvalue _returnvalue_2))
  (bind _returnvalue_4 (Math|Vector|VectorLength _returnvalue_3))
  (bind _returnvalue_5 (/ _returnvalue_4 _distanceorigine))
  (bind _returnvalue_6 (* _origin_scale _returnvalue_5))
  (if (Variables|Default|GetIs%20grabbed%20?)
    (Transformation|SetWorldScale3D (Variables|/Game/Blueprint/BP_PlanetPhysics.BP_PlanetPhysics_C|GetSphere (Variables|Default|GetAs%20BP%20Planet%20Physics)) (Math|Vector|MakeVector (Math|Float|Clamp(Float) (.x _returnvalue_6) (Variables|Default|GetMin) (Variables|Default|GetMax)) (Math|Float|Clamp(Float) (.y _returnvalue_6) (Variables|Default|GetMin) (Variables|Default|GetMax)) (Math|Float|Clamp(Float) (.z _returnvalue_6) (Variables|Default|GetMin) (Variables|Default|GetMax))))))

(fn ConstructionScript)