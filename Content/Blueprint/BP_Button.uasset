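; BP_Button is a physical XR button whose cylinder moves along local Z while a motion controller visualization component overlaps its box.
; Each linked tick projects the controller's displacement onto DirectionBouton and adds its unsigned length to Z, clamped between PositionMin and PositionMax.
; Reaching a limit calls the empty ActionMin or ActionMax hook.
; Overlap end unlinks the controller and optionally snaps the cylinder to a limit chosen by IsOn.
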(event OnComponentBeginOverlap(Box)
  (params (OverlappedComponent :type Primitive%20Component%20Object%20Reference) (OtherActor :type Actor%20Object%20Reference) (OtherComp :type Primitive%20Component%20Object%20Reference) (OtherBodyIndex :type Integer) (bFromSweep :type Boolean) (SweepResult :type Hit%20Result%20Structure%20%28by%20ref%29))
  ;[1 1 1] On récupère le motion controller qui appuie sur le bouton
  (bind _asxrdevice_visualization_component (Utilities|Casting|CastToXRDeviceVisualizationComponent OtherComp))
  (Variables|Default|SetIsLinked true)
  (Variables|Default|SetMotionController _asxrdevice_visualization_component)
  ;[1 1 1] On Prend la première position pour plus tard
  (Variables|Default|SetPosN (Transformation|GetWorldLocation _asxrdevice_visualization_component)))

(event OnComponentEndOverlap(Box)
  (params (OverlappedComponent :type Primitive%20Component%20Object%20Reference) (OtherActor :type Actor%20Object%20Reference) (OtherComp :type Primitive%20Component%20Object%20Reference) (OtherBodyIndex :type Integer))
  (bind _cylinder (Variables|Default|GetCylinder))
  ;[1 1 1] On sépare le motion controller du bouton et on le remet à sa position initiale si l'option est cochée
  (Utilities|Casting|CastToXRDeviceVisualizationComponent OtherComp)
  (Variables|Default|SetIsLinked false)
  (if (Variables|Default|GetRetourPosInitiale)
    (if (Variables|Default|GetIsOn)
      (Transformation|SetRelativeLocation _cylinder (Math|Vector|MakeVector 0.0 0.0 (Variables|Default|GetPositionMin)) false false)
      (else
        (Transformation|SetRelativeLocation _cylinder (Math|Vector|MakeVector 0.0 0.0 (Variables|Default|GetPositionMax)) false false)))))

(event EventTick
  (params (DeltaSeconds :type Float%20%28single-precision%29))
  (bind _cylinder (Variables|Default|GetCylinder))
  (if (Variables|Default|GetIsLinked)
    (CallFunction|CalculDelta)
    ;[1 1 1] On regarde quelle sera la prochaine position du bouton par rapport au delta
    (bind _deltabutton (CallFunction|ProjectionDelta))
    (Variables|Default|SetnextExpectedLocation (+ _deltabutton (.z (Variables|/Script/Engine.SceneComponent|GetRelativeLocation (Variables|Default|GetCylinder)))))
    ;[1 1 1] Si le bouton est relevé plus haut que son maximum, il s'arrête au maximum et déclencle l'action Max
    (if (>= (Variables|Default|GetnextExpectedLocation) (Variables|Default|GetPositionMax))
      (Transformation|SetRelativeLocation _cylinder (Math|Vector|MakeVector 0.0 0.0 (Variables|Default|GetPositionMax)) false false)
      (CallFunction|ActionMax)
      (else
        ;[1 1 1] Si il est enfoncé plus loin que son minimum, il s'arrête au minimun et déclanche l'action Min
        (if (<= (Variables|Default|GetnextExpectedLocation) (Variables|Default|GetPositionMin))
          (Transformation|SetRelativeLocation _cylinder (Math|Vector|MakeVector 0.0 0.0 (Variables|Default|GetPositionMin)) false false)
          (CallFunction|ActionMin)
          (else
            ;[1 1 1] Sinon, il se déplace vers la prochaine position prévue
            (Transformation|AddRelativeLocation _cylinder (Math|Vector|MakeVector 0.0 0.0 _deltabutton) false false)))))))

(fn ConstructionScript)

(fn CalculDelta
  (bind _motioncontroller (Variables|Default|GetMotionController))
  (bind _returnvalue (Transformation|GetWorldLocation _motioncontroller))
  ;[1 1 1] On Soustrait la position précédente à la position actuelle pour avoir le déplacement
  (Variables|Default|SetDelta (- (Variables|Default|GetPosN) _returnvalue))
  (Variables|Default|SetPosN _returnvalue)
  (return))

(fn ProjectionDelta
  (return (Math|Vector|VectorLength (Math|Vector|ProjectVectorontoVector (Variables|Default|GetDelta) (Variables|Default|GetDirectionBouton)))))

(fn ActionMin)

(fn ActionMax)