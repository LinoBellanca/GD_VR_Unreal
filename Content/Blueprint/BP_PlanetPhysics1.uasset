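; VR-grabbable planet that, once dropped, is pulled toward BP_GravityCenter by an acceleration growing linearly with distance.
; Grabbing pauses that pull and attaches a BP_GrabExt resize handle to the other hand.
; While inactive, sphere scale switches it between random rock and planet, choosing material and asteroid count.
; A distance-based hot/cold Niagara switch is unfinished: IsHot is only set false and both branches use snow.
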(event OnDropped(GrabComponent)
  ;[1 0.007073 0] Physique
  ;;[1 1 1] Se charge tout seul de l'inertie
  (Variables|Default|SetIsActive true)
  (Actor|DestroyActor (Variables|Default|GetGrab%20Ext%20ref)))

(event OnGrabbed(GrabComponent)
  ;[0 0.0192 1] Aggrandissement
  ;;[1 1 1] On désacctive la physique et détruit la poignée d'aggrandissement
  (Variables|Default|SetIsActive false)
  (Utilities|IsValid (Variables|Default|GetGrab%20Ext%20ref)
    (:Is%20Valid
      (Actor|DestroyActor (Variables|Default|GetGrab%20Ext%20ref)))
    (:Is%20Not%20Valid
      _))
  ;;[1 1 1] On regarde dans quelle main on tient la planète
  (bind _returnvalue (Actor|GetActorOfClass "/Game/VRTemplate/Blueprints/VRPawn.VRPawn_C"))
  ;;[1 1 1] On fixe une poignée d'aggrandissement à l'autre main
  (if (== (Variables|/Game/VRTemplate/Blueprints/VRPawn.VRPawn_C|GetMotionControllerLeft _returnvalue) (Variables|/Game/VRTemplate/Blueprints/GrabComponent.GrabComponent_C|GetMotionControllerRef (Variables|Default|GetGrabComponent)))
    (bind _returnvalue_2 (Game|SpawnActorfromClass "/Game/Blueprint/BP_GrabExt.BP_GrabExt_C" (Transformation|GetWorldTransform (Variables|/Game/VRTemplate/Blueprints/VRPawn.VRPawn_C|GetMotionControllerRight _returnvalue)) "AlwaysSpawn" "MultiplyWithRoot" 0 self 0 0))
    (Transformation|AttachComponentToComponent _returnvalue_2 (Variables|/Game/VRTemplate/Blueprints/VRPawn.VRPawn_C|GetMotionControllerRight _returnvalue) "None" "SnapToTarget" "KeepWorld" "KeepWorld" true)
    (Variables|Default|SetGrab%20Ext%20ref _returnvalue_2)
    (else
      (bind _returnvalue_3 (Game|SpawnActorfromClass "/Game/Blueprint/BP_GrabExt.BP_GrabExt_C" (Transformation|GetWorldTransform (Variables|/Game/VRTemplate/Blueprints/VRPawn.VRPawn_C|GetMotionControllerLeft _returnvalue)) "AlwaysSpawn" "MultiplyWithRoot" 0 self 0 0))
      (Transformation|AttachComponentToComponent _returnvalue_3 (Variables|/Game/VRTemplate/Blueprints/VRPawn.VRPawn_C|GetMotionControllerLeft _returnvalue) "None" "SnapToTarget" "KeepWorld" "KeepWorld" true)
      (Variables|Default|SetGrab%20Ext%20ref _returnvalue_3))))

(event Custom|UpdateNiagara
  (if (Variables|Default|GetIs%20Hot%20?)
    (Class|NiagaraComponent|SetAsset (Variables|Default|GetNiagara) "/Game/Blueprint/Niagara/NS_Snow.NS_Snow" true)
    (else
      ;[0 1 0.05424] Skin+Mesh
      (Class|NiagaraComponent|SetAsset (Variables|Default|GetNiagara) "/Game/Blueprint/Niagara/NS_Snow.NS_Snow" true))))

(event EventTick
  (params (DeltaSeconds :type Float%20%28single-precision%29))
  (bind _sphere (Variables|Default|GetSphere))
  (bind _gravitycenter (Variables|Default|GetGravityCenter))
  (bind _sphere_2 (Variables|Default|GetSphere))
  (bind _returnvalue (Transformation|GetWorldScale _sphere_2))
  (bind _returnvalue_2 (Transformation|GetActorLocation _gravitycenter))
  (bind _returnvalue_3 (Transformation|GetWorldLocation _sphere))
  (bind _returnvalue_4 (- _returnvalue_2 _returnvalue_3))
  ;[1 0.007073 0] Physique
  ;;[1 1 1] Gravité
  (if (Variables|Default|GetIsActive)
    (Variables|Default|SetDistance%20avec%20soleil _returnvalue_4)
    (Physics|AddForce _sphere (* _returnvalue_4 (Variables|Default|GetGravityStrength)) "None" true)
    (if (>= (Math|Vector|VectorLength (Variables|Default|GetDistance%20avec%20soleil)) 3e+03)
      (if (Variables|Default|GetIs%20Hot%20?)
        (Variables|Default|SetIs%20Hot%20? false)
        ;[0 0.0192 1] Aggrandissement
        ;;[1 1 1] On désacctive la physique et détruit la poignée d'aggrandissement
        (CallFunction|UpdateNiagara :!label _label))
      (elif (not (Variables|Default|GetIs%20Hot%20?))
        (Variables|Default|SetIs%20Hot%20? false)
        (goto _label)))
    (else
      ;[0 1 0.05424] Skin+Mesh
      ;;[1 1 1] False = on reste un astéroide / True = devient planète
      (Utilities|FlowControl|Delay 0.1)
      ;;;[1 1 1] Update du visuel
      (if (Math|Boolean|ANDBoolean (>= (.x _returnvalue) 0.2) (>= (.y _returnvalue) 0.2) (>= (.z _returnvalue) 0.2))
        (Rendering|SetVisibility (Variables|Default|GetStaticMesh) false false)
        (Rendering|SetVisibility (Variables|Default|GetSphere) true false)
        (Variables|Default|SetAsteroidsSpawned 5)
        ;;[1 1 1] Material en fct de la taille
        (if (>= (.z _returnvalue) 0.3)
          (if (>= (.z _returnvalue) 0.4)
            (if (>= (.z _returnvalue) 0.5)
              (if (>= (.z _returnvalue) 0.6)
                (if (>= (.z _returnvalue) 0.7)
                  (if (>= (.z _returnvalue) 0.8)
                    (if (>= (.z _returnvalue) 0.9)
                      (if (>= (.z _returnvalue) 1.0)
                        (Variables|Default|SetIntMAT 7)
                        (Rendering|Material|SetMaterial (Variables|Default|GetSphere) 0 (Utilities|Array|Get(acopy) (Variables|Default|GetMAT_planetes) (Variables|Default|GetIntMAT)) :!label _label_2))
                      (else
                        (Variables|Default|SetIntMAT 6)
                        (goto _label_2)))
                    (else
                      (Variables|Default|SetIntMAT 5)
                      (goto _label_2)))
                  (else
                    (Variables|Default|SetIntMAT 4)
                    (goto _label_2)))
                (else
                  (Variables|Default|SetIntMAT 3)
                  (goto _label_2)))
              (else
                (Variables|Default|SetIntMAT 2)
                (goto _label_2)))
            (else
              (Variables|Default|SetIntMAT 1)
              (goto _label_2)))
          (else
            (Variables|Default|SetIntMAT 0)
            (goto _label_2)))
        (else
          (Rendering|SetVisibility (Variables|Default|GetStaticMesh) true false)
          (Rendering|SetVisibility (Variables|Default|GetSphere) false false)
          (Variables|Default|SetAsteroidsSpawned 0))))))

(event EventBeginPlay
  ;[1 0.007073 0] Physique
  ;;[1 1 1] Point d'attraction
  (bind _returnvalue (Actor|GetActorOfClass "/Game/Blueprint/BP_GravityCenter.BP_GravityCenter_C"))
  (Variables|Default|SetGravityCenter _returnvalue)
  (Collision|SetActorEnableCollision self true))

(fn ConstructionScript
  (Components|StaticMesh|SetStaticMesh (Variables|Default|GetStaticMesh) (Utilities|Array|Get(acopy) (Variables|Default|Getmeshcailloux) (Math|Random|RandomInteger 6))))