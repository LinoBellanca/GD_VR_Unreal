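; BP_Planet is a planet actor that spins at a constant rate around its vertical axis.
; On BeginPlay it finds and stores the level's BP_GravityCenter, moves Sphere1 to that actor's location and places Sphere at InitialPos.
; Tick advances the whole actor's yaw, scaled by delta time for frame-rate independence, with no physics or gravity calculation.
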(event EventBeginPlay
  (bind _returnvalue (Actor|GetActorOfClass "/Game/Blueprint/BP_GravityCenter.BP_GravityCenter_C"))
  (bind _output_get (Variables|Default|SetGravityCenter _returnvalue))
  (Transformation|SetWorldLocation (Variables|Default|GetSphere1) (Transformation|GetActorLocation _output_get) false false)
  (Transformation|SetWorldLocation (Variables|Default|GetSphere) (Variables|Default|GetInitialPos) false false))

(event EventTick
  (params (DeltaSeconds :type Float%20%28single-precision%29))
  (Transformation|SetActorRotation (Math|Rotator|MakeRotator 0.0 0.0 (+ (.yaw (Transformation|GetActorRotation)) (* DeltaSeconds 5.0)))))

(fn ConstructionScript)