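; VR-grabbable planet that starts as a random rock mesh and is pulled toward BP_GravityCenter when active.
; Grabbing pauses gravity and spawns a BP_GrabExt on the other controller; dropping destroys it and reactivates gravity.
; While inactive, delayed Tick checks swap the rock for a sphere above a scale threshold and pick its material by size.
; Gravity is an acceleration force growing linearly with distance, relying on inertia for orbits.
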(event OnDropped(GrabComponent)
  ;[1 1 1] Physique
  ;;[1 1 1] Se charge tout seul de l'inertie
  (Variables|Default|SetIsActive true)
  (Actor|DestroyActor (Variables|Default|GetGrab%20Ext%20ref)))

(event OnGrabbed(GrabComponent)
  (Variables|Default|SetIsActive false)
  (bind _returnvalue (Actor|GetActorOfClass "/Game/VRTemplate/Blueprints/VRPawn.VRPawn_C"))
  (if (== (Variables|/Game/VRTemplate/Blueprints/VRPawn.VRPawn_C|GetMotionControllerLeft _returnvalue) (Variables|/Game/VRTemplate/Blueprints/GrabComponent.GrabComponent_C|GetMotionControllerRef (Variables|Default|GetGrabComponent)))
    (bind _returnvalue_2 (Game|SpawnActorfromClass "/Game/Blueprint/BP_GrabExt.BP_GrabExt_C" (Transformation|GetWorldTransform (Variables|/Game/VRTemplate/Blueprints/VRPawn.VRPawn_C|GetMotionControllerRight _returnvalue)) "AlwaysSpawn" "MultiplyWithRoot" 0 self 0 0))
    (Transformation|AttachComponentToComponent _returnvalue_2 (Variables|/Game/VRTemplate/Blueprints/VRPawn.VRPawn_C|GetMotionControllerRight _returnvalue) "None" "SnapToTarget" "KeepWorld" "KeepWorld" true)
    (Variables|Default|SetGrab%20Ext%20ref _returnvalue_2)
    (else
      (bind _returnvalue_3 (Game|SpawnActorfromClass "/Game/Blueprint/BP_GrabExt.BP_GrabExt_C" (Transformation|GetWorldTransform (Variables|/Game/VRTemplate/Blueprints/VRPawn.VRPawn_C|GetMotionControllerLeft _returnvalue)) "AlwaysSpawn" "MultiplyWithRoot" 0 self 0 0))
      (Transformation|AttachComponentToComponent _returnvalue_3 (Variables|/Game/VRTemplate/Blueprints/VRPawn.VRPawn_C|GetMotionControllerLeft _returnvalue) "None" "SnapToTarget" "KeepWorld" "KeepWorld" true)
      (Variables|Default|SetGrab%20Ext%20ref _returnvalue_3))))

(event EventTick
  (params (DeltaSeconds :type Float%20%28single-precision%29))
  (bind _sphere (Variables|Default|GetSphere))
  (bind _sphere_2 (Variables|Default|GetSphere))
  (bind _returnvalue (Transformation|GetWorldScale _sphere_2))
  ;[1 1 1] Physique
  (if (Variables|Default|GetIsActive)
    (Physics|AddForce _sphere (* (- (Transformation|GetActorLocation (Variables|Default|GetGravityCenter)) (Transformation|GetWorldLocation _sphere)) (Variables|Default|GetGravityStrength)) "None" true)
    (else
      (Utilities|FlowControl|Delay 0.1)
      (if (Math|Boolean|ANDBoolean (>= (.x _returnvalue) 0.2) (>= (.y _returnvalue) 0.2) (>= (.z _returnvalue) 0.2))
        (Rendering|SetVisibility (Variables|Default|GetStaticMesh) false false)
        (Rendering|SetVisibility (Variables|Default|GetSphere) true false)
        (if (>= (.z _returnvalue) 0.3)
          (if (>= (.z _returnvalue) 0.4)
            (if (>= (.z _returnvalue) 0.5)
              (if (>= (.z _returnvalue) 0.6)
                (if (>= (.z _returnvalue) 0.7)
                  (if true
                    (if (>= (.z _returnvalue) 0.9)
                      (if (>= (.z _returnvalue) 1.0)
                        (Variables|Default|SetIntMAT 7)
                        (Rendering|Material|SetMaterial (Variables|Default|GetSphere) 0 (Utilities|Array|Get(acopy) (Variables|Default|GetMAT_planetes) (Variables|Default|GetIntMAT)) :!label _label))
                      (else
                        (Variables|Default|SetIntMAT 6)
                        (goto _label)))
                    (else
                      (Variables|Default|SetIntMAT 5)
                      (goto _label)))
                  (else
                    (Variables|Default|SetIntMAT 4)
                    (goto _label)))
                (else
                  (Variables|Default|SetIntMAT 3)
                  (goto _label)))
              (else
                (Variables|Default|SetIntMAT 2)
                (goto _label)))
            (else
              (Variables|Default|SetIntMAT 1)
              (goto _label)))
          (else
            (Variables|Default|SetIntMAT 0)
            (goto _label)))))))

(event EventBeginPlay
  ;[1 1 1] Physique
  (bind _returnvalue (Actor|GetActorOfClass "/Game/Blueprint/BP_GravityCenter.BP_GravityCenter_C"))
  (Variables|Default|SetGravityCenter _returnvalue))

(fn ConstructionScript
  (Components|StaticMesh|SetStaticMesh (Variables|Default|GetStaticMesh) (Utilities|Array|Get(acopy) (Variables|Default|Getmeshcailloux) (Math|Random|RandomInteger 6))))